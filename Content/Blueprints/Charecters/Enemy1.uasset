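; Enemy character that spawns with two swords and chases the player character Tom when it sees him.
; On BeginPlay it attaches the swords to two mesh sockets, and PawnSensing drives an AI MoveTo toward Tom while it is alive.
; Damage from other actors lowers health in the CharecterInfo struct, playing a hit montage or setting the dead flag with a death montage.
; The attack montage is unconnected and HitOccur is empty.
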(event `self.ReceiveBeginPlay`
  (`parent.ReceiveBeginPlay`)
  (`self.SpawnWeapon`))

(event `self.PawnSensing.OnSeePawn`
  (params (Pawn :type "Pawn Object Reference"))
  (bind (_charecterinfo_currenthealth _charecterinfo_currentenergy _charecterinfo_isdead) (break `/Game/Blueprints/Charecters/CharecterInfo_Struct` (`self.CharecterInfo`)))
  (bind _astom (cast `/Game/Blueprints/Charecters/Tom` Pawn))
  (if (not _charecterinfo_isdead)
    (`|AIMoveTo` self (0.0 0.0 0.0) _astom 100.0 true)))

(event `self.ReceiveAnyDamage`
  (params (Damage :type "Float (single-precision)") (DamageType :type "DamageType Object Reference") (InstigatedBy :type "Controller Object Reference") (DamageCauser :type "Actor Object Reference"))
  (bind (_charecterinfo_currenthealth _charecterinfo_currentenergy _charecterinfo_isdead _charecterinfo_type _charecterinfo_maxhealth _charecterinfo_maxenergy) (break `/Game/Blueprints/Charecters/CharecterInfo_Struct` (`self.CharecterInfo`)))
  (bind _returnvalue (- _charecterinfo_currenthealth Damage))
  (if (and (!= DamageCauser self) (not _charecterinfo_isdead))
    (if (<= _returnvalue 0.0)
      (set `self.CharecterInfo` (make `/Game/Blueprints/Charecters/CharecterInfo_Struct` 0.0 _charecterinfo_currentenergy true _charecterinfo_type _charecterinfo_maxhealth _charecterinfo_maxenergy))
      (bind _returnvalue_2 (`self.PlayAnimMontage` "/Game/Assets/TwinbladesAnimsetBase/RootMotion/Twinblades_Dead_Montage.Twinblades_Dead_Montage"))
      (`KismetSystemLibrary.Delay` _returnvalue_2)
      (else
        (set `self.CharecterInfo` (make `/Game/Blueprints/Charecters/CharecterInfo_Struct` _returnvalue _charecterinfo_currentenergy false _charecterinfo_type _charecterinfo_maxhealth _charecterinfo_maxenergy))
        (bind _returnvalue_3 (`self.PlayAnimMontage` "/Game/Assets/TwinbladesAnimsetBase/RootMotion/Player_Hit_Front_AM.Player_Hit_Front_AM"))
        (`KismetSystemLibrary.Delay` _returnvalue_3)))))

(fn `HitOccur`)

(fn `SpawnWeapon`
  (bind _returnvalue (`|SpawnActorFromClass` "/Game/Blueprints/Weapon/Sword.Sword_C" (`self.GetTransform`) "Undefined" "OverrideRootScale" null null))
  (`self.K2_AttachToComponent` _returnvalue (`self.Mesh`) "W1" "SnapToTarget" "SnapToTarget" "SnapToTarget" true)
  (bind _returnvalue_2 (`|SpawnActorFromClass` "/Game/Blueprints/Weapon/Sword.Sword_C" (`self.GetTransform`) "Undefined" "OverrideRootScale" null null))
  (`self.K2_AttachToComponent` _returnvalue_2 (`self.Mesh`) "W2" "SnapToTarget" "SnapToTarget" "SnapToTarget" true))

(fn `UserConstructionScript`
  (`parent.UserConstructionScript`))