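; Game instance Blueprint for Crestscendo that acts as a central hub for showing the game's menu screens.
; Separate events show the main menu, settings, load and loading screens, plus the in-game menu, settings, save and load widgets.
; Each event creates its widget for player 0 only if the cached reference is invalid, then adds it to the viewport.
; A helper function converts a level enum value to a Name.
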(event `ShowInGameMenu`
  ;[1 1 1] Show In Game Menu
  (`/Engine/EditorBlueprintResources/StandardMacros.IsValid` (`self.MenuIGWidget`)
    (:`Is Valid`
      _)
    (:`Is Not Valid`
      (bind _returnvalue (`|CreateWidget` "/Game/UI/InGame/Menu_IG.Menu_IG_C" (`GameplayStatics.GetPlayerController` 0)))
      (set `self.MenuIGWidget` _returnvalue)))
  (`UserWidget.AddToViewport` (`self.MenuIGWidget`) 0))

(event `ShowMainMenu`
  ;[1 1 1] Show Main Menu Widget
  (`/Engine/EditorBlueprintResources/StandardMacros.IsValid` (`self.MainMenuWidget`)
    (:`Is Valid`
      _)
    (:`Is Not Valid`
      (bind _returnvalue (`|CreateWidget` "/Game/UI/Menu/MainMenu.MainMenu_C" (`GameplayStatics.GetPlayerController` 0)))
      (set `self.MainMenuWidget` _returnvalue)))
  (`UserWidget.AddToViewport` (`self.MainMenuWidget`) 0))

(event `ShowSettings`
  ;[1 1 1] Show Settings Widget
  (`/Engine/EditorBlueprintResources/StandardMacros.IsValid` (`self.SettingsWidget`)
    (:`Is Valid`
      _)
    (:`Is Not Valid`
      (bind _returnvalue (`|CreateWidget` "/Game/UI/Menu/Settings.Settings_C" (`GameplayStatics.GetPlayerController` 0)))
      (set `self.SettingsWidget` _returnvalue)))
  (`UserWidget.AddToViewport` (`self.SettingsWidget`) 0))

(event `ShowInGameLoad`
  ;[1 1 1] Show In Game Load
  (`/Engine/EditorBlueprintResources/StandardMacros.IsValid` (`self.LoadIgWidget`)
    (:`Is Valid`
      _)
    (:`Is Not Valid`
      (bind _returnvalue (`|CreateWidget` "/Game/UI/InGame/LoadGame_IG.LoadGame_IG_C" (`GameplayStatics.GetPlayerController` 0)))
      (set `self.LoadIgWidget` _returnvalue)))
  (`UserWidget.AddToViewport` (`self.LoadIgWidget`) 0))

(event `ShowLoadGame`
  ;[1 1 1] Show Load Game Widget
  (`/Engine/EditorBlueprintResources/StandardMacros.IsValid` (`self.LoadGameWidget`)
    (:`Is Valid`
      _)
    (:`Is Not Valid`
      (bind _returnvalue (`|CreateWidget` "/Game/UI/Menu/LoadGame.LoadGame_C" (`GameplayStatics.GetPlayerController` 0)))
      (set `self.LoadGameWidget` _returnvalue)))
  (`UserWidget.AddToViewport` (`self.LoadGameWidget`) 0))

(event `ShowInGameSave`
  ;[1 1 1] Show In Game Save
  (`/Engine/EditorBlueprintResources/StandardMacros.IsValid` (`self.SaveWidget`)
    (:`Is Valid`
      _)
    (:`Is Not Valid`
      (bind _returnvalue (`|CreateWidget` "/Game/UI/InGame/SaveGame.SaveGame_C" (`GameplayStatics.GetPlayerController` 0)))
      (set `self.SaveWidget` _returnvalue)))
  (`UserWidget.AddToViewport` (`self.SaveWidget`) 0))

(event `Show Loading Screen`
  ;[1 1 1] Show Loading Screen
  (`/Engine/EditorBlueprintResources/StandardMacros.IsValid` (`self.LoadingScreenWidget`)
    (:`Is Valid`
      _)
    (:`Is Not Valid`
      (bind _returnvalue (`|CreateWidget` "/Game/UI/LoadingScreen.LoadingScreen_C" (`GameplayStatics.GetPlayerController` 0)))
      (set `self.LoadingScreenWidget` _returnvalue)))
  (`UserWidget.AddToViewport` (`self.LoadingScreenWidget`) 0))

(event `ShowInGameSettings`
  ;[1 1 1] Show In Game Settings
  (`/Engine/EditorBlueprintResources/StandardMacros.IsValid` (`self.SettingsIGWidget`)
    (:`Is Valid`
      _)
    (:`Is Not Valid`
      (bind _returnvalue (`|CreateWidget` "/Game/UI/InGame/Settings_IG.Settings_IG_C" (`GameplayStatics.GetPlayerController` 0)))
      (set `self.SettingsIGWidget` _returnvalue)))
  (`UserWidget.AddToViewport` (`self.SettingsIGWidget`) 0))

(fn `Cast_ELevelToName`
  (params (LevelName :type "/Game/Levels/LevenNameEnum Enum" :default "NewEnumerator0"))
  (returns (Name :type Name))
  (return (`KismetStringLibrary.Conv_StringToName` (`|GetEnumeratorNameAsString` LevelName))))